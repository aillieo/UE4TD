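; Base AI controller for tower defence enemies that spawns its own enemy pawn and sends it along the path.
; On BeginPlay it caches the TDGameMode, spawns a BP_Enemy_Base at the first path point and possesses it.
; It then uses AI MoveTo toward the second path point only, printing a debug string on success, with no handling of further points yet.
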(event `self.ReceiveBeginPlay`
  (`self.CacheGameMode`)
  (`self.CreateEnemyAndMove`))

(fn `CacheGameMode`
  (bind _astdgame_mode (cast `/Game/TowerDefence/Blueprints/TDGameMode` (`GameplayStatics.GetGameMode`)))
  (set `self.TDGameMode` _astdgame_mode))

(fn `UserConstructionScript`)