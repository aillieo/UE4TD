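; Tower defence game mode that sets up a test path and spawns a single enemy when play begins.
; InitPathPoints spawns a straight row of evenly spaced BP_PathPoint actors along X and stores them in the PathPoints array.
; After a short delay, BeginPlay spawns one BP_Enemy_Base just above the world origin, where the row starts.
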(event `self.ReceiveBeginPlay`
  (`self.InitPathPoints`)
  (`KismetSystemLibrary.Delay` 5.0)
  (`|SpawnActorFromClass` "/Game/TowerDefence/Blueprints/Enemy/BP_Enemy_Base.BP_Enemy_Base_C" (`KismetMathLibrary.MakeTransform` (0.0 0.0 100.0)) "AdjustIfPossibleButAlwaysSpawn" "OverrideRootScale" null null))

(fn `InitPathPoints`
  (for _index (range 6)
    (bind _returnvalue (`|SpawnActorFromClass` "/Game/TowerDefence/Blueprints/BP_PathPoint.BP_PathPoint_C" (`KismetMathLibrary.MakeTransform` (`KismetMathLibrary.MakeVector` (* _index 500.0))) "Undefined" "OverrideRootScale" null null))
    (`KismetArrayLibrary.Array_Add` (`self.PathPoints`) _returnvalue)))

(fn `UserConstructionScript`)