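; Player controller for a tower defence game that spawns and possesses a TDCharacter on BeginPlay and moves it around the level with WASD.
; Each key press sets a fixed axis-aligned velocity and a move flag, and releasing any of the keys clears the flag.
; Tick offsets the pawn's location by that velocity scaled by delta time, without sweeping, so only the last pressed direction applies and diagonals are not supported.
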(event `self.ReceiveBeginPlay`
  (bind _returnvalue (`|SpawnActorFromClass` "/Game/TowerDefence/Blueprints/TDCharacter.TDCharacter_C" (`KismetMathLibrary.MakeTransform` (0.0 0.0 100.0)) "Undefined" "OverrideRootScale" null null))
  (`self.Possess` _returnvalue))

(event `self.ReceiveTick`
  (params (DeltaSeconds :type "Float (single-precision)"))
  (bind _returnvalue (`self.K2_GetPawn`))
  (if (`self.CamMove`)
    (`self.K2_SetActorLocation` _returnvalue (+ (* (`self.CamMoveSpeed`) DeltaSeconds) (`self.K2_GetActorLocation` _returnvalue)) false false)))

(event `Key|A`
  (params (Key :type "Key Structure"))
  (:`Pressed`
    (set `self.CamMoveSpeed` (-400.0 0.0 0.0))
    (set `self.CamMove` true :!label _label))
  (:`Released`
    (set `self.CamMove` false :!label _label_2)))

(event `Key|D`
  (params (Key :type "Key Structure"))
  (:`Pressed`
    (set `self.CamMoveSpeed` (400.0 0.0 0.0))
    (goto _label))
  (:`Released`
    (goto _label_2)))

(event `Key|W`
  (params (Key :type "Key Structure"))
  (:`Pressed`
    (set `self.CamMoveSpeed` (0.0 -400.0 0.0))
    (goto _label))
  (:`Released`
    (goto _label_2)))

(event `Key|S`
  (params (Key :type "Key Structure"))
  (:`Pressed`
    (set `self.CamMoveSpeed` (0.0 400.0 0.0))
    (goto _label))
  (:`Released`
    (goto _label_2)))

(fn `UserConstructionScript`)